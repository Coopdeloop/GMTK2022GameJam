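; BP_ShopManager runs the shop in a board game, handling the menu and item purchases.
; OpenShop resets the player's root rotation, then creates the W_ShopMenu widget and enables mouse input for it.
; Buy charges the game mode's current-turn player and adds the item to their linked character's inventory, destroying the item if gold is short.
; CloseShopMenu calls FinishLand on the shop space to end the visit.
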(event `self.ReceiveBeginPlay`)

(event `Open Shop`
  (params (Player :type "/Game/Blueprints/Character/BoardCharacters/BP_BoardBaseCharacter Object Reference") (`Shop Space` :type "/Game/Blueprints/Spaces/BP_BoardSpace Object Reference"))
  (`SceneComponent.K2_SetRelativeRotation` (`Actor.RootComponent` Player) (`self.rotator`) false false)
  (`self.Open Shop Menu` `Shop Space`))

(event `Open Shop Menu`
  (params (ShopSpace :type "/Game/Blueprints/Spaces/BP_BoardSpace Object Reference"))
  (bind _returnvalue (`GameplayStatics.GetPlayerController` 0))
  (bind _returnvalue_2 (`|CreateWidget` "/Game/UI/w_ShopMenu.w_ShopMenu_C"))
  (`UserWidget.AddToViewport` _returnvalue_2 0)
  (`WidgetBlueprintLibrary.SetInputMode_GameAndUIEx` _returnvalue null "DoNotLock" false)
  (set `PlayerController.bShowMouseCursor` true _returnvalue)
  (`KismetSystemLibrary.PrintString` "Menu Open")
  (if (`/Game/UI/w_ShopMenu.Exit` _returnvalue_2)
    (set `self.exited` true)))

(event `Close Shop Menu`
  (`/Game/Blueprints/Spaces/BP_BoardSpace.FinishLand` (stale `Open Shop Menu` ShopSpace))
  (`KismetSystemLibrary.PrintString` "Next Turn"))

(fn `Buy`
  (params (cost :type Integer) (item :type "/Game/Blueprints/Items/BP_Base_Item Object Reference"))
  (bind _item (`self.Item`))
  (bind _cost (`self.Cost`))
  (set `self.Item` item)
  (bind _returnvalue (`GameplayStatics.GetActorOfClass` "/Game/Blueprints/BP_BoardGameMode.BP_BoardGameMode_C"))
  (bind _curplayerturn (`/Game/Blueprints/BP_BoardGameMode.CurPlayerTurn` _returnvalue))
  (bind _output_get (set `self.Player` _curplayerturn))
  (set `self.Cost` cost)
  (if (>= (`/Game/Blueprints/Character/BoardCharacters/BP_BoardBaseCharacter.CurGold` _output_get) _cost)
    (`/Game/Blueprints/Character/BoardCharacters/BP_BoardBaseCharacter.SpendGold` (`self.Player`) _cost)
    (`KismetSystemLibrary.PrintString` "Item Bought")
    (`/Game/Blueprints/Character/ActionCharacters/BP_Inventory.AddItem` (`/Game/Blueprints/Character/ActionCharacters/BP_ActionBaseCharacter.BP_Inventory` (`/Game/Blueprints/Character/BoardCharacters/BP_BoardBaseCharacter.LinkedActionCharacter` _curplayerturn)) _item)
    (`KismetSystemLibrary.PrintString` "Item Added")
    (else
      (`KismetSystemLibrary.PrintString` "Not Enough Gold")
      (`self.K2_DestroyActor` _item))))

(fn `UserConstructionScript`)