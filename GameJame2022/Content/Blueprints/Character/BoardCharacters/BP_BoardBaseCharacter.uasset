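; Base board-game character that runs a player's turn: menu, dice roll, movement along board spaces, landing and turn handoff.
; A successful roll from BP_DiceManager activates any active item and sets a modified step count, which DecrementMovement consumes using BP_BoardManager's next-space lookup.
; Each step uses SimpleMoveToActor with a looping timeline animating the piece mesh.
; The final space's landing callback ends the turn through the game mode; gold helpers track currency.
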(event `self.ReceiveBeginPlay`
  (bind _returnvalue (`GameplayStatics.GetActorOfClass` "/Game/Blueprints/Spaces/BP_BoardManager.BP_BoardManager_C"))
  (set `self.BoardManager` _returnvalue)
  (bind _returnvalue_2 (`GameplayStatics.GetActorOfClass` "/Game/Blueprints/Dice/BP_DiceManager.BP_DiceManager_C"))
  (set `self.DiceManager` _returnvalue_2)
  (`TimelineComponent.SetPlayRate` (`self.MovingTimeline`) 3.0)
  (set `self.MeshStartPos` (`SceneComponent.RelativeLocation` (`self.PlayerPiece`))))

(event `StartTurn`
  (`KismetSystemLibrary.Delay` 2.0)
  (bind _returnvalue (`|CreateWidget` "/Game/UI/w_PlayerMenu.w_PlayerMenu_C" null self))
  (`UserWidget.AddToViewport` _returnvalue 0))

(event `DecrementMovement`
  (`TimelineComponent.SetLooping` (`self.MovingTimeline`) false)
  (if (> (`self.RemainingSpaces`) 0)
    (`/Engine/EditorBlueprintResources/StandardMacros.DecrementInt` (`self.RemainingSpaces`)
      (:`  `
        (bind _newboardspace (`/Game/Blueprints/Spaces/BP_BoardManager.GetNextBoardSpace` (`self.BoardManager`) (`self.CurSpace`)))
        (set `self.CurSpace` _newboardspace)
        (`KismetSystemLibrary.Delay` 0.1)
        (`self.MoveCharacter`)))
    (else
      (`KismetSystemLibrary.Delay` 1.0)
      (`self.SpaceLogic`)
      (remove `/Game/Blueprints/Dice/BP_DiceManager.OnSuccessfulRoll` (`self.DiceManager`) (delegate `StartMoving`)))))

(event `MoveCharacter`
  (`AIBlueprintHelperLibrary.SimpleMoveToActor` (`self.GetController`) (`self.CurSpace`))
  (`TimelineComponent.SetLooping` (`self.MovingTimeline`) true)
  (bind (_direction _staticmeshlocation) (`Timeline|MovingTimeline`)
    (:`Update`
      (`SceneComponent.K2_SetRelativeLocation` (`self.PlayerPiece`) (+ _staticmeshlocation (`self.MeshStartPos`)) false false))))

(event `EndTurn`
  (bind _asbp_board_game_mode (cast `/Game/Blueprints/BP_BoardGameMode` (`GameplayStatics.GetGameMode`)))
  (`/Game/Blueprints/BP_BoardGameMode.NextTurn` _asbp_board_game_mode))

(event `Roll`
  (bind _dicemanager (`self.DiceManager`))
  (add `/Game/Blueprints/Dice/BP_DiceManager.OnSuccessfulRoll` _dicemanager (delegate `StartMoving`))
  (`/Game/Blueprints/BP_BoardGameMode.EnterDiceThrowStart` (cast `/Game/Blueprints/BP_BoardGameMode` (`GameplayStatics.GetGameMode`) :!pure true))
  (`KismetSystemLibrary.Delay` 0.5)
  (`/Game/Blueprints/Dice/BP_DiceManager.RollDice` _dicemanager))

(event `StartMoving`
  (params (TotalValue :type Integer))
  (bind _activeitems (`self.ActiveItems`))
  (bind _dicemanager (`self.DiceManager`))
  (bind _movespaces (`self.MoveSpaces`))
  (`/Engine/EditorBlueprintResources/StandardMacros.IsValid` _activeitems
    (:`Is Valid`
      (`/Game/Blueprints/Items/BP_Base_Item.ActivateItem` _activeitems))
    (:`Is Not Valid`
      _))
  (bind _output_get (set `self.MoveSpaces` (+ (`/Game/Blueprints/Dice/BP_DiceManager.TotalValue` _dicemanager) (`/Game/Blueprints/Dice/BP_DiceManager.RollModifier` _dicemanager))))
  (if (< _output_get 1)
    (set `self.MoveSpaces` 1))
  (`KismetSystemLibrary.PrintString` (`KismetStringLibrary.Conv_IntToString` _movespaces))
  (set `self.RemainingSpaces` _movespaces)
  (`/Game/Blueprints/BP_BoardGameMode.EnterMovementStart` (cast `/Game/Blueprints/BP_BoardGameMode` (`GameplayStatics.GetGameMode`) :!pure true))
  (`KismetSystemLibrary.Delay` 1.0)
  (`self.DecrementMovement`))

(event `SpaceLogic`
  (add `/Game/Blueprints/Spaces/BP_BoardSpace.FinishedLanding` (`self.CurSpace`) (delegate `FinishedLanding`))
  (`/Game/Blueprints/Spaces/BP_BoardSpace.Landed` (`self.CurSpace`) self))

(event `FinishedLanding`
  (`KismetSystemLibrary.Delay` 1.0)
  (`self.EndTurn`))

(fn `AddGold`
  (params (AddedGold :type Integer))
  (set `self.CurGold` (+ (`self.CurGold`) AddedGold)))

(fn `SpendGold`
  (params (SpentGold :type Integer))
  (bind _returnvalue (- (`self.CurGold`) SpentGold))
  (set `self.CurGold` (`KismetMathLibrary.SelectInt` 0 _returnvalue (< _returnvalue 0))))

(fn `UserConstructionScript`)