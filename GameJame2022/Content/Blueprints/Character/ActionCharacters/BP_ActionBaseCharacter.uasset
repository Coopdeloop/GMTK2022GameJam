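; Base character Blueprint for action characters, deriving its combat stats from equipped gear.
; On BeginPlay it asks its BPInventory to give starting gear, then runs SetStats.
; SetStats sums attack, defense, health and speed across the head, chest, leg and weapon slots.
; LevelUp is an empty stub.
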(event `self.ReceiveBeginPlay`
  (`/Game/Blueprints/Character/ActionCharacters/BP_Inventory.Give Starting Gear` (`self.BP_Inventory`))
  (`self.Set Stats`))

(fn `Level Up`)

(fn `Set Stats`
  (bind _bp_inventory (`self.BP_Inventory`))
  (bind _head_slot (`/Game/Blueprints/Character/ActionCharacters/BP_Inventory.Head Slot` _bp_inventory))
  (bind _chest_slot (`/Game/Blueprints/Character/ActionCharacters/BP_Inventory.Chest Slot` _bp_inventory))
  (bind _leg_slot (`/Game/Blueprints/Character/ActionCharacters/BP_Inventory.Leg Slot` _bp_inventory))
  (bind _weapon_slot (`/Game/Blueprints/Character/ActionCharacters/BP_Inventory.Weapon Slot` _bp_inventory))
  (set `self.ATK` (+ (`/Game/Blueprints/Gear/BP_Base_Equipment.Gear_ATK` _head_slot) (`/Game/Blueprints/Gear/BP_Base_Equipment.Gear_ATK` _chest_slot) (`/Game/Blueprints/Gear/BP_Base_Equipment.Gear_ATK` _leg_slot) (`/Game/Blueprints/Gear/BP_Base_Equipment.Gear_ATK` _weapon_slot)))
  (set `self.DEF` (+ (`/Game/Blueprints/Gear/BP_Base_Equipment.Gear_DEF` _head_slot) (`/Game/Blueprints/Gear/BP_Base_Equipment.Gear_DEF` _chest_slot) (`/Game/Blueprints/Gear/BP_Base_Equipment.Gear_DEF` _leg_slot) (`/Game/Blueprints/Gear/BP_Base_Equipment.Gear_DEF` _weapon_slot)))
  (set `self.HP` (+ (`/Game/Blueprints/Gear/BP_Base_Equipment.Gear_HP` _head_slot) (`/Game/Blueprints/Gear/BP_Base_Equipment.Gear_HP` _chest_slot) (`/Game/Blueprints/Gear/BP_Base_Equipment.Gear_HP` _leg_slot) (`/Game/Blueprints/Gear/BP_Base_Equipment.Gear_HP` _weapon_slot)))
  (set `self.SPD` (+ (`/Game/Blueprints/Gear/BP_Base_Equipment.Gear_SPD` _head_slot) (`/Game/Blueprints/Gear/BP_Base_Equipment.Gear_SPD` _chest_slot) (`/Game/Blueprints/Gear/BP_Base_Equipment.Gear_SPD` _leg_slot) (`/Game/Blueprints/Gear/BP_Base_Equipment.Gear_SPD` _weapon_slot))))

(fn `UserConstructionScript`)