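; Inventory for action characters, holding head, chest, leg and weapon gear plus separate board and battle item lists.
; Each Assign function destroys the slot's old actor, stores the new one and calls SetStats on the owning BP_ActionBaseCharacter.
; GiveStartingGear spawns and equips basic armor, adding a wooden stick for the Warrior class.
; AddItem routes Consumable items to the board list and Movement Buff items to the battle list.
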(fn `AddBattleItem`
  (params (Item :type "/Game/Blueprints/Items/BP_Base_Item Object Reference"))
  (`KismetArrayLibrary.Array_Add` (`self.BattleItems`) Item))

(fn `AddBoardItem`
  (params (Item :type "/Game/Blueprints/Items/BP_Base_Item Object Reference"))
  (`KismetArrayLibrary.Array_Add` (`self.Board Items`) Item))

(fn `AddItem`
  (params (ItemToAdd :type "/Game/Blueprints/Items/BP_Base_Item Object Reference"))
  (bind (_s_item_itemname _s_item_itemicon _s_item_itemtype) (break `/Game/Blueprints/Items/S_Item` (`/Game/Blueprints/Items/BP_Base_Item.S_Item` ItemToAdd)))
  (switch `/Game/Blueprints/Items/E_ItemType` _s_item_itemtype
    (:`NewEnumerator0`
      (`self.AddBoardItem` ItemToAdd))
    (:`NewEnumerator2`
      (`self.AddBattleItem` ItemToAdd))))

(fn `Assign Chest`
  (params (`New Chest` :type "/Game/Blueprints/Gear/Chest/BP_Base_Chest Object Reference"))
  (`Actor.K2_DestroyActor` (`self.Chest Slot`))
  (set `self.Chest Slot` `New Chest`)
  (bind _asbp_action_base_character (cast `/Game/Blueprints/Character/ActionCharacters/BP_ActionBaseCharacter` (`self.GetOwner`)))
  (`/Game/Blueprints/Character/ActionCharacters/BP_ActionBaseCharacter.Set Stats` _asbp_action_base_character))

(fn `Assign Head`
  (params (`New Helm` :type "/Game/Blueprints/Gear/Helm/BP_Base_Helm Object Reference"))
  (`Actor.K2_DestroyActor` (`self.Head Slot`))
  (set `self.Head Slot` `New Helm`)
  (bind _asbp_action_base_character (cast `/Game/Blueprints/Character/ActionCharacters/BP_ActionBaseCharacter` (`self.GetOwner`)))
  (`/Game/Blueprints/Character/ActionCharacters/BP_ActionBaseCharacter.Set Stats` _asbp_action_base_character))

(fn `Assign Legs`
  (params (`New Legs` :type "/Game/Blueprints/Gear/Legs/BP_Base_Legs Object Reference"))
  (`Actor.K2_DestroyActor` (`self.Leg Slot`))
  (set `self.Leg Slot` `New Legs`)
  (bind _asbp_action_base_character (cast `/Game/Blueprints/Character/ActionCharacters/BP_ActionBaseCharacter` (`self.GetOwner`)))
  (`/Game/Blueprints/Character/ActionCharacters/BP_ActionBaseCharacter.Set Stats` _asbp_action_base_character))

(fn `Assign Weapon`
  (params (`New Weapon` :type "/Game/Blueprints/Gear/Weapon/BP_Base_Weapon Object Reference"))
  (`Actor.K2_DestroyActor` (`self.Weapon Slot`))
  (set `self.Weapon Slot` `New Weapon`)
  (bind _asbp_action_base_character (cast `/Game/Blueprints/Character/ActionCharacters/BP_ActionBaseCharacter` (`self.GetOwner`)))
  (`/Game/Blueprints/Character/ActionCharacters/BP_ActionBaseCharacter.Set Stats` _asbp_action_base_character))

(fn `DiscardBattleItem`
  (params (Item :type "/Game/Blueprints/Items/BP_Base_Item Object Reference"))
  (`KismetArrayLibrary.Array_RemoveItem` (`self.BattleItems`) Item))

(fn `DiscardBoardItem`
  (params (Item :type "/Game/Blueprints/Items/BP_Base_Item Object Reference"))
  (`KismetArrayLibrary.Array_RemoveItem` (`self.Board Items`) Item))

(fn `Give Starting Gear`
  (bind _returnvalue (`self.GetOwner`))
  (bind _returnvalue_2 (`Actor.GetTransform` _returnvalue))
  (bind _returnvalue_3 (`|SpawnActorFromClass` "/Game/Blueprints/Gear/Helm/BP_Cap.BP_Cap_C" _returnvalue_2 "Undefined" "OverrideRootScale" null null))
  (`self.Assign Head` _returnvalue_3)
  (bind _returnvalue_4 (`|SpawnActorFromClass` "/Game/Blueprints/Gear/Chest/BP_Tattered_Shirt.BP_Tattered_Shirt_C" _returnvalue_2 "Undefined" "OverrideRootScale" null null))
  (`self.Assign Chest` _returnvalue_4)
  (bind _returnvalue_5 (`|SpawnActorFromClass` "/Game/Blueprints/Gear/Legs/BP_Torn_Pants.BP_Torn_Pants_C" _returnvalue_2 "Undefined" "OverrideRootScale" null null))
  (`self.Assign Legs` _returnvalue_5)
  (bind _asbp_action_base_character (cast `/Game/Blueprints/Character/ActionCharacters/BP_ActionBaseCharacter` _returnvalue))
  (switch `/Game/Blueprints/Character/E_PlayerClass` (`/Game/Blueprints/Character/ActionCharacters/BP_ActionBaseCharacter.eClass` _asbp_action_base_character)
    (:`NewEnumerator0`
      (bind _returnvalue_6 (`|SpawnActorFromClass` "/Game/Blueprints/Gear/Weapon/BP_T1_Wooden_Stick.BP_T1_Wooden_Stick_C" _returnvalue_2 "Undefined" "OverrideRootScale" null null))
      (`self.Assign Weapon` _returnvalue_6))))