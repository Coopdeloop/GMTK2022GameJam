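; BP_DiceBoostSmall_Item is a usable item that gives a small flat boost to a dice roll.
; UseItem calls the parent, prints a message and registers the item with BP_DiceManager as used.
; ActivateItem applies the bonus through the manager's ModifyRoll, separating use from effect.
; Both functions find the manager with GetActorOfClass, and the ItemEffect event is empty.
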(event `ItemEffect`)

(fn `ActivateItem`
  (bind _returnvalue (`GameplayStatics.GetActorOfClass` "/Game/Blueprints/Dice/BP_DiceManager.BP_DiceManager_C"))
  (`/Game/Blueprints/Dice/BP_DiceManager.ModifyRoll` _returnvalue 3))

(fn `UseItem`
  (`parent.UseItem`)
  (`KismetSystemLibrary.PrintString` "Add +3 to roll")
  (bind _returnvalue (`GameplayStatics.GetActorOfClass` "/Game/Blueprints/Dice/BP_DiceManager.BP_DiceManager_C"))
  (`/Game/Blueprints/Dice/BP_DiceManager.AddUsedItem` _returnvalue self))

(fn `UserConstructionScript`
  (`parent.UserConstructionScript`))