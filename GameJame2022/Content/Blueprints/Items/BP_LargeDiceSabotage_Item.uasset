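; Board game sabotage item that subtracts 4 from another player's dice roll.
; UseItem calls the parent, prints the effect and adds the item to the ActiveItems of the player at hardcoded index 1 in BP_BoardGameMode.
; ActivateItem later applies the penalty to RollModifier on BP_DiceManager.
; Both managers are found with GetActorOfClass, and the ItemEffect event is empty.
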(event `ItemEffect`)

(fn `ActivateItem`
  (bind _returnvalue (`GameplayStatics.GetActorOfClass` "/Game/Blueprints/Dice/BP_DiceManager.BP_DiceManager_C"))
  (set `/Game/Blueprints/Dice/BP_DiceManager.RollModifier` (+ (`/Game/Blueprints/Dice/BP_DiceManager.RollModifier` _returnvalue) -4) _returnvalue))

(fn `UseItem`
  (`parent.UseItem`)
  (`KismetSystemLibrary.PrintString` "Subtracts 4 from another player's roll")
  (bind _returnvalue (`GameplayStatics.GetActorOfClass` "/Game/Blueprints/BP_BoardGameMode.BP_BoardGameMode_C"))
  (`KismetArrayLibrary.Array_Add` (`/Game/Blueprints/Character/BoardCharacters/BP_BoardBaseCharacter.ActiveItems` (`|GetArrayItem` (`/Game/Blueprints/BP_BoardGameMode.Players` _returnvalue) 1)) self))

(fn `UserConstructionScript`
  (`parent.UserConstructionScript`))