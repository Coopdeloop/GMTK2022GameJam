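; A landable space that starts a battle between the landing character and a grunt.
; OnLanded finds the BP_BattlePhaseManager, sets the character's LinkedActionCharacter as Player1, spawns a BP_Grunt at the space's transform as Player2 and calls BattleStart.
; It binds to the manager's OnBattleFinished only after starting the battle.
; FinishLand calls the parent implementation, then removes that binding.
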(fn `FinishLand`
  (`parent.FinishLand`)
  (remove `/Game/Blueprints/Battle/BP_BattlePhaseManager.OnBattleFinished` (`self.BattlePhaseManager`) (`|CreateDelegate` :!event `FinishLand`)))

(fn `OnLanded`
  (params (Character :type "/Game/Blueprints/Character/BoardCharacters/BP_BoardBaseCharacter Object Reference"))
  (bind _battlephasemanager (`self.BattlePhaseManager`))
  (bind _returnvalue (`GameplayStatics.GetActorOfClass` "/Game/Blueprints/Battle/BP_BattlePhaseManager.BP_BattlePhaseManager_C"))
  (set `self.BattlePhaseManager` _returnvalue)
  (set `/Game/Blueprints/Battle/BP_BattlePhaseManager.Player1` (`/Game/Blueprints/Character/BoardCharacters/BP_BoardBaseCharacter.LinkedActionCharacter` Character) (`self.BattlePhaseManager`))
  (bind _returnvalue_2 (`|SpawnActorFromClass` "/Game/Blueprints/Character/ActionCharacters/BP_Grunt.BP_Grunt_C" (`self.GetTransform`) "Undefined" "OverrideRootScale" null null))
  (set `/Game/Blueprints/Battle/BP_BattlePhaseManager.Player2` _returnvalue_2 (`self.BattlePhaseManager`))
  (`/Game/Blueprints/Battle/BP_BattlePhaseManager.BattleStart` _battlephasemanager)
  (add `/Game/Blueprints/Battle/BP_BattlePhaseManager.OnBattleFinished` _battlephasemanager (`|CreateDelegate` :!event `FinishLand`)))

(fn `UserConstructionScript`
  (`parent.UserConstructionScript`))