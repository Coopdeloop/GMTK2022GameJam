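; BP_ShopSpace is a space that opens a shop when a character lands on it.
; On BeginPlay it spawns a BP_Shop at its own transform composed with ShopLocation, then turns itself to a fixed diagonal yaw.
; OnLanded finds the BP_ShopManager in the level and calls OpenShop, passing the landing character and itself.
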(event `self.ReceiveBeginPlay`
  (`|SpawnActorFromClass` "/Game/Blueprints/Shop/BP_Shop.BP_Shop_C" (`KismetMathLibrary.ComposeTransforms` (`self.GetTransform`) (`self.shop location`)) "Undefined" "OverrideRootScale" null null)
  (`self.K2_SetActorRotation` (`KismetMathLibrary.Conv_VectorToRotator` (1.0 1.0 0.0))))

(fn `OnLanded`
  (params (Character :type "/Game/Blueprints/Character/BoardCharacters/BP_BoardBaseCharacter Object Reference"))
  (bind _returnvalue (`GameplayStatics.GetActorOfClass` "/Game/Blueprints/Shop/BP_ShopManager.BP_ShopManager_C"))
  (set `self.ShopManager` _returnvalue)
  (bind _output_get (set `self.shopspace` self))
  (`/Game/Blueprints/Shop/BP_ShopManager.Open Shop` (`self.ShopManager`) Character _output_get))

(fn `UserConstructionScript`
  (`parent.UserConstructionScript`))