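; Base board space for a board game, providing overridable hooks for characters that pass or land on it.
; When a character whose current space is this one enters the trigger box, a short delay precedes Passed, which decrements its movement and calls OnPassed.
; Landed calls OnLanded, whose default immediately calls FinishLand.
; FinishLand fires the FinishedLanding dispatcher, then unbinds all listeners, making each subscription one-shot.
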(event `Landed`
  (params (Character :type "/Game/Blueprints/Character/BoardCharacters/BP_BoardBaseCharacter Object Reference"))
  (`self.OnLanded` Character))

(event `Passed`
  (params (Character :type "/Game/Blueprints/Character/BoardCharacters/BP_BoardBaseCharacter Object Reference"))
  (`/Game/Blueprints/Character/BoardCharacters/BP_BoardBaseCharacter.DecrementMovement` Character)
  (`self.OnPassed` Character))

(event `self.TriggerBox.OnComponentBeginOverlap`
  (params (OverlappedComponent :type "PrimitiveComponent Object Reference") (OtherActor :type "Actor Object Reference") (OtherComp :type "PrimitiveComponent Object Reference") (OtherBodyIndex :type Integer) (bFromSweep :type Boolean) (SweepResult :type "HitResult Structure (by ref)"))
  (bind _asbp_board_base_character (cast `/Game/Blueprints/Character/BoardCharacters/BP_BoardBaseCharacter` OtherActor))
  (if (== (`/Game/Blueprints/Character/BoardCharacters/BP_BoardBaseCharacter.CurSpace` _asbp_board_base_character) self)
    (`KismetSystemLibrary.Delay` 0.1)
    (`self.Passed` _asbp_board_base_character)))

(fn `FinishLand`
  (`self.FinishedLanding`)
  (clear `self.FinishedLanding`))

(fn `OnLanded`
  (params (Character :type "/Game/Blueprints/Character/BoardCharacters/BP_BoardBaseCharacter Object Reference"))
  ;[1 1 1] Custom Implementation per space
  (`self.FinishLand`))

(fn `OnPassed`
  (params (Character :type "/Game/Blueprints/Character/BoardCharacters/BP_BoardBaseCharacter Object Reference"))
  ;[1 1 1] Custom Implementation per space
)

(fn `UserConstructionScript`)