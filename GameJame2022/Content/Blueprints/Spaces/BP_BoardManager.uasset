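; Board manager actor that builds a randomized game board of space actors at BeginPlay.
; For each SpaceLocations entry, RollSpace draws a random type from BoardSpaceAmounts, spawns it scaled up at that actor-relative offset, and appends it to BoardSpaces.
; Each draw decrements that type's remaining amount, removing exhausted types from the pool.
; GetNextBoardSpace returns the following array entry; its wrap-to-zero check uses > Length, so the last space indexes out of range.
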(event `RollSpace`
  (params (BoardSpaceToProduce :type Integer))
  (bind (_output_spacetype _output_amount) (break `/Game/Blueprints/Spaces/S_BoardSpaceAmounts` (`|GetArrayItem` (`self.BoardSpaceAmounts`) BoardSpaceToProduce)))
  (if (> _output_amount 0)
    (bind _result (`/Engine/EditorBlueprintResources/StandardMacros.DecrementInt` _output_amount)
      (:`  `
        (`|ExecutionSequence`
          (:`then_0`
            (bind _returnvalue (`|SpawnActorFromClass` _output_spacetype (`KismetMathLibrary.MakeTransform` (+ (stale `self.ReceiveBeginPlay` _array_element) (`self.K2_GetActorLocation`)) (struct) (4.0 4.0 4.0)) "Undefined" "OverrideRootScale" null null))
            (`KismetArrayLibrary.Array_Add` (`self.BoardSpaces`) _returnvalue))
          (:`then_1`
            (if (<= _result 0)
              (`KismetArrayLibrary.Array_Remove` (`self.BoardSpaceAmounts`) BoardSpaceToProduce))))))))

(event `self.ReceiveBeginPlay`
  (for _array_element (`self.SpaceLocations`)
    (`self.RollSpace` (`KismetMathLibrary.RandomIntegerInRange` 0 (- (`KismetArrayLibrary.Array_Length` (`self.BoardSpaceAmounts`)) 1)))))

(fn `GetNextBoardSpace`
  (params (CurrentBoardSpace :type "/Game/Blueprints/Spaces/BP_BoardSpace Object Reference"))
  (returns (NewBoardSpace :type "/Game/Blueprints/Spaces/BP_BoardSpace Object Reference"))
  (bind _returnvalue (+ (`KismetArrayLibrary.Array_Find` (`self.BoardSpaces`) CurrentBoardSpace) 1))
  (return (`|GetArrayItem` (`self.BoardSpaces`) (`KismetMathLibrary.SelectInt` 0 _returnvalue (> _returnvalue (`KismetArrayLibrary.Array_Length` (`self.BoardSpaces`)))))))

(fn `UserConstructionScript`)