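; Camera manager for the board game that switches the player's view between character, overview, dice and battle shots.
; It registers itself with BP_BoardGameMode on BeginPlay and exposes an event per shot that calls SetViewTargetWithBlend on the first player controller.
; A separate event re-attaches PlayerCamera at an offset from the current character, while the player shot targets the Character itself.
; The dice shot sets only a blend exponent, with no blend time.
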(event `self.ReceiveBeginPlay`
  (bind _asbp_board_game_mode (cast `/Game/Blueprints/BP_BoardGameMode` (`GameplayStatics.GetGameMode`)))
  (set `/Game/Blueprints/BP_BoardGameMode.CameraManager` self _asbp_board_game_mode))

(event `SetCameraToCurrentCharacter`
  (params (Character :type "/Game/Blueprints/Character/BoardCharacters/BP_BoardBaseCharacter Object Reference"))
  (bind _playercamera (`self.PlayerCamera`))
  (`self.K2_DetachFromActor` _playercamera "KeepRelative" "KeepRelative" "KeepRelative")
  (`self.K2_SetActorLocation` _playercamera (+ (`self.K2_GetActorLocation` Character) (-225.0 0.0 175.0)) false false)
  (`self.K2_AttachToActor` _playercamera Character "None" "KeepRelative" "KeepRelative" "KeepRelative" true))

(event `GoToPlayerCamera`
  (params (Character :type "/Game/Blueprints/Character/BoardCharacters/BP_BoardBaseCharacter Object Reference"))
  (`PlayerController.SetViewTargetWithBlend` (`GameplayStatics.GetPlayerController` 0) Character 0.5 "VTBlend_Linear" 0.0 false))

(event `GoToOverviewCamera`
  (`PlayerController.SetViewTargetWithBlend` (`GameplayStatics.GetPlayerController` 0) (`self.OverviewCamera`) 0.5 "VTBlend_Linear" 0.0 false))

(event `GoToDiceCamera`
  (`PlayerController.SetViewTargetWithBlend` (`GameplayStatics.GetPlayerController` 0) (`self.DiceCamera`) 0.0 "VTBlend_Linear" 0.5 false))

(event `GoToBattleCamera`
  (`PlayerController.SetViewTargetWithBlend` (`GameplayStatics.GetPlayerController` 0) (`self.BattleCamera`) 0.5 "VTBlend_Linear" 0.0 false))

(fn `UserConstructionScript`)