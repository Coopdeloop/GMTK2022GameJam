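; Game mode for a turn-based board game that spawns players, cycles turns and switches cameras by phase.
; After startup delays, it spawns up to four human characters at player starts, then starts the first turn with a mouse cursor.
; NextTurn wraps through Players, counting rounds, while phase events direct CameraManager to overview, dice, player or battle views.
; ShowResults creates the results widget; random turn-order shuffling exists but is disconnected.
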(event `self.ReceiveBeginPlay`
  (`KismetSystemLibrary.Delay` 2.0)
  (`self.PopulatePlayers`))

(event `StartGame`
  (bind _returnvalue (`GameplayStatics.GetPlayerController` 0))
  (bind _output_get (set `self.CurPlayerTurn` (`|GetArrayItem` (`self.Players`))))
  (set `self.CurGlobalTurn` 1)
  (`/Game/Blueprints/Character/BoardCharacters/BP_BoardBaseCharacter.StartTurn` _output_get)
  (`self.EnterTurnStart`)
  (`WidgetBlueprintLibrary.SetInputMode_UIOnlyEx` _returnvalue null)
  (set `PlayerController.bShowMouseCursor` true _returnvalue))

(event `NextTurn`
  (bind _players (`self.Players`))
  (bind _returnvalue (+ (`KismetArrayLibrary.Array_Find` _players (`self.CurPlayerTurn`)) 1))
  (bind _returnvalue_2 (>= _returnvalue (`KismetArrayLibrary.Array_Length` _players)))
  (if _returnvalue_2
    (`/Engine/EditorBlueprintResources/StandardMacros.IncrementInt` (`self.CurGlobalTurn`)
      (:`  `
        _)))
  (bind _output_get (set `self.CurPlayerTurn` (`|GetArrayItem` (`self.Players`) (`KismetMathLibrary.SelectInt` 0 _returnvalue _returnvalue_2))))
  (`/Game/Blueprints/Character/BoardCharacters/BP_BoardBaseCharacter.StartTurn` _output_get)
  (`self.EnterTurnStart`))

(event `PopulatePlayers`
  (`|ExecutionSequence`
    (:`then_0`
      (bind _outactors (`GameplayStatics.GetAllActorsOfClass` "/Game/Blueprints/Spaces/BP_PlayerStart.BP_PlayerStart_C"))
      (for _index (range 4)
        (if (< _index (`self.HumanPlayerAmount`))
          (bind _output (`|GetArrayItem` _outactors _index))
          (bind (_returnvalue_location _returnvalue_rotation _returnvalue_scale) (`KismetMathLibrary.BreakTransform` (`self.GetTransform` _output)))
          (bind _returnvalue (`|SpawnActorFromClass` "/Game/Blueprints/Character/BoardCharacters/BP_BoardBaseCharacter.BP_BoardBaseCharacter_C" (`KismetMathLibrary.MakeTransform` (`SceneComponent.K2_GetComponentLocation` (`/Game/Blueprints/Spaces/BP_PlayerStart.PlayerStartPos` _output)) _returnvalue_rotation _returnvalue_scale) "Undefined" "OverrideRootScale" null null))
          (`KismetArrayLibrary.Array_Add` (`self.Players`) _returnvalue))))
    (:`then_1`
      (`KismetSystemLibrary.Delay` 2.0)
      (`self.StartGame`))))

(event `EnterTurnStart`
  (`/Game/Blueprints/CameraWork/BP_CameraManager.GoToOverviewCamera` (`self.CameraManager`)))

(event `ShowResults`
  (`|CreateWidget` "/Game/UI/w_Results.w_Results_C" null (`self.Players`)))

(event `EnterDiceThrowStart`
  (`/Game/Blueprints/CameraWork/BP_CameraManager.GoToDiceCamera` (`self.CameraManager`)))

(event `EnterMovementStart`
  (`/Game/Blueprints/CameraWork/BP_CameraManager.GoToPlayerCamera` (`self.CameraManager`) (`self.CurPlayerTurn`)))

(event `EnterBattleStart`
  (`/Game/Blueprints/CameraWork/BP_CameraManager.GoToBattleCamera` (`self.CameraManager`)))

(fn `AddToOrder`
  (params (Order :type "Array of /Game/Blueprints/Character/BoardCharacters/BP_BoardBaseCharacter Object Reference"))
  (bind _output (`|GetArrayItem` (`self.Players`) (`KismetMathLibrary.RandomIntegerInRange` 0 (- (`KismetArrayLibrary.Array_Length` (`self.Players`)) 1))))
  (`KismetArrayLibrary.Array_Add` Order _output)
  (`KismetArrayLibrary.Array_RemoveItem` (`self.Players`) _output)
  (if (< (`KismetArrayLibrary.Array_Length` (`self.Players`)) 1)
    _))

(fn `DetermineTurnOrder`
  (locals (PlayerOrder :type "Array of /Game/Blueprints/Character/BoardCharacters/BP_BoardBaseCharacter Object Reference"))
  (bind _playerorder (`local.PlayerOrder`))
  (for _ (range 4)
    (`self.AddToOrder` _playerorder))
  (bind _output_get (set `self.Players` _playerorder))
  (for _array_element _output_get
    (`KismetSystemLibrary.PrintString` (`KismetSystemLibrary.GetObjectName` _array_element) true true (struct :`R` 0.986793 :`G` 1.0 :`A` 1.0) 4.0)))

(fn `UserConstructionScript`)