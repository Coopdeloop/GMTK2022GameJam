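; Dice manager actor that spawns physical dice, rolls them with an impulse and totals their results.
; Each die reports through a bound OnRolled event; after the last one and a short delay, queued items activate and OnSuccessfulRoll broadcasts the total.
; It then destroys the dice and clears used items and the roll modifier, which is accumulated but never added to the total here.
; Holding Space speeds up global time.
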(event `CalculateRoll`
  (params (NumRolled :type Integer))
  (set `self.TotalValue` (+ (`self.TotalValue`) NumRolled))
  (`/Engine/EditorBlueprintResources/StandardMacros.IncrementInt` (`self.CurrentlyRolled`)
    (:`  `
      (if (>= (`self.CurrentlyRolled`) (`KismetArrayLibrary.Array_Length` (`self.DiceInUse`)))
        (`KismetSystemLibrary.Delay` 1.5)
        (`self.AfterRollEffects`)
        (`KismetSystemLibrary.PrintString` (`KismetStringLibrary.Conv_IntToString` (`self.TotalValue`)))
        (`self.OnSuccessfulRoll` (`self.TotalValue`))
        (for _array_element (`self.DiceInUse`)
          (`self.K2_DestroyActor` _array_element))
        (`KismetArrayLibrary.Array_Clear` (`self.DiceInUse`))
        (`self.EndOfRoll`)))))

(event `BindDice`
  (for _array_element (`self.DiceInUse`)
    (add `/Game/Blueprints/Dice/BP_Die.OnRolled` _array_element (delegate `CalculateRoll`))))

(event `RollDice`
  (bind (_returnvalue_location _returnvalue_rotation _returnvalue_scale) (`KismetMathLibrary.BreakTransform` (`self.GetTransform`)))
  (for _index (range (`self.AmountOfDice`))
    (bind _returnvalue (`|SpawnActorFromClass` (select `int` _index :`0` "/Game/Blueprints/Dice/BP_Die.BP_Die_C" :`1` "/Game/Blueprints/Dice/BP_DieMagicPattern.BP_DieMagicPattern_C" :!type "Actor Class Reference") (`KismetMathLibrary.MakeTransform` (+ _returnvalue_location (`KismetMathLibrary.MakeVector` 0.0 0.0 (`KismetMathLibrary.Conv_IntToDouble` (* _index 100)))) _returnvalue_rotation _returnvalue_scale) "Undefined" "OverrideRootScale" null null))
    (`KismetArrayLibrary.Array_Add` (`self.DiceInUse`) (cast `/Game/Blueprints/Dice/BP_Die` _returnvalue :!pure true)))
  (`self.BindDice`)
  (set `self.TotalValue` 0)
  (for _array_element (`self.DiceInUse`)
    (bind _returnvalue_2 (`KismetMathLibrary.SelectFloat` 100.0 -100.0 (== _index 0)))
    (`/Game/Blueprints/Dice/BP_Die.Roll die` :`self` _array_element :`ImpulseDirection` (+ (`self.StandardImpulse`) (`KismetMathLibrary.MakeVector` _returnvalue_2 _returnvalue_2)))))

(event `Key|SpaceBar`
  (params (Key :type "Key Structure"))
  (:`Pressed`
    (`GameplayStatics.SetGlobalTimeDilation` 5.0))
  (:`Released`
    (`GameplayStatics.SetGlobalTimeDilation` 1.0)))

(event `self.ReceiveBeginPlay`
  (`self.EnableInput` (`GameplayStatics.GetPlayerController` 0)))

(fn `AddUsedItem`
  (params (NewParam :type "/Game/Blueprints/Items/BP_Base_Item Object Reference"))
  (`KismetArrayLibrary.Array_Add` (`self.UsedItems`) NewParam))

(fn `AfterRollEffects`
  (for _array_element (`self.UsedItems`)
    (`KismetSystemLibrary.PrintString` (`.ItemName_9_FA8C800C4765B6C3076A0DB4B441D523` (break `/Game/Blueprints/Items/S_Item` (`/Game/Blueprints/Items/BP_Base_Item.S_Item` _array_element))) true true (struct :`R` 1.0 :`B` 0.617563 :`A` 1.0))
    (`/Game/Blueprints/Items/BP_Base_Item.ActivateItem` _array_element)))

(fn `EndOfRoll`
  (set `self.RollModifier` 0)
  (`KismetArrayLibrary.Array_Clear` (`self.UsedItems`)))

(fn `ModifyRoll`
  (params (Input :type Integer))
  (set `self.RollModifier` (+ (`self.RollModifier`) Input)))

(fn `UserConstructionScript`)