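; BP_Die is a physics die that is thrown by an impulse, detects when it settles, and reports the number rolled.
; Rolldie enables gravity, applies the impulse plus random torque, then starts a looping timer that polls the cube's velocity.
; Once it slows, CalculateRoll finds the child TextRender facing world up and parses its text as the result, broadcast through OnRolled.
; ResetPosition returns the die to its starting location.
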(event `self.ReceiveBeginPlay`
  (`PrimitiveComponent.SetEnableGravity` (`self.Cube`) false)
  (set `self.StartPos` (`self.K2_GetActorLocation`)))

(event `CheckIfStoppedRolling`
  (if (<= (`KismetMathLibrary.VSize` (`SceneComponent.GetComponentVelocity` (`self.Cube`))) 25.0)
    (`KismetSystemLibrary.K2_ClearAndInvalidateTimerHandle` (stale `Roll die` _returnvalue_2))
    (`self.Rolled`)))

(event `Roll die`
  (params (ImpulseDirection :type "Vector Structure"))
  (bind _cube (`self.Cube`))
  (bind _returnvalue (* (`KismetMathLibrary.RandomFloatInRange` 25000.0 40000.0) (`KismetMathLibrary.SelectFloat` 1.0 -1.0 (`KismetMathLibrary.RandomBool`))))
  (`PrimitiveComponent.SetEnableGravity` (`self.Cube`) true)
  (`PrimitiveComponent.AddImpulse` _cube ImpulseDirection "None" true)
  (`PrimitiveComponent.AddTorqueInDegrees` _cube (`KismetMathLibrary.MakeVector` _returnvalue _returnvalue _returnvalue) "None" true)
  (bind _returnvalue_2 (`KismetSystemLibrary.K2_SetTimerDelegate` (delegate `CheckIfStoppedRolling`) 0.25 true 2.0)))

(event `ResetPosition`
  (`self.K2_SetActorLocation` (`self.StartPos`)))

(event `Rolled`
  (`KismetSystemLibrary.Delay` 0.5)
  (`self.CalculateRoll`)
  (`KismetSystemLibrary.PrintString` (`KismetStringLibrary.Concat_StrStr` "Rolled A " (`KismetStringLibrary.Conv_IntToString` (`self.NumRolled`))) true true (struct :`R` 1.0 :`G` 0.880592 :`A` 1.0) 4.0)
  (`self.OnRolled` (`self.NumRolled`)))

(fn `CalculateRoll`
  (for _array_element (`SceneComponent.GetChildrenComponents` (`self.Cube`) false)
    (if (== (`KismetMathLibrary.GetUpVector` (struct)) (`SceneComponent.GetForwardVector` _array_element))
      (bind _astext_render_component (cast `TextRenderComponent` _array_element))
      (set `self.NumRolled` (`KismetStringLibrary.Conv_StringToInt` (`KismetTextLibrary.Conv_TextToString` (`TextRenderComponent.Text` _astext_render_component))))
      (break))))

(fn `UserConstructionScript`)