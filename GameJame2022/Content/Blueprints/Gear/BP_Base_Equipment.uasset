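; Base actor for clickable loot gear (helm, chest, legs, weapon) in a board game with battle phases.
; On BeginPlay it rolls HP, ATK, DEF and SPD within ranges and fills a hidden LootPanel widget, marking each stat +, - or / against the current player's equipped item.
; Clicking assigns it to that character's inventory slot, refreshes stats, moves it below the board and removes it from the battle manager's destroy list.
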(event `self.ReceiveActorOnClicked`
  (params (ButtonPressed :type "Key Structure"))
  (bind (_s_gear_icon _s_gear_name _s_gear_geartype) (break `/Game/Blueprints/Gear/S_GearBase` (`self.S_Gear`)))
  (bind _asbp_board_game_mode (cast `/Game/Blueprints/BP_BoardGameMode` (`GameplayStatics.GetGameMode`)))
  (switch `/Game/Blueprints/Gear/E_GearType` _s_gear_geartype
    (:`NewEnumerator0`
      (bind _asbp_base_helm (cast `/Game/Blueprints/Gear/Helm/BP_Base_Helm` self))
      (bind _linkedactioncharacter (`/Game/Blueprints/Character/BoardCharacters/BP_BoardBaseCharacter.LinkedActionCharacter` (`/Game/Blueprints/BP_BoardGameMode.CurPlayerTurn` _asbp_board_game_mode)))
      (bind _returnvalue (`self.GetComponentByClass` _linkedactioncharacter "/Game/Blueprints/Character/ActionCharacters/BP_Inventory.BP_Inventory_C"))
      (`/Game/Blueprints/Character/ActionCharacters/BP_Inventory.Assign Head` _returnvalue _asbp_base_helm))
    (:`NewEnumerator1`
      (bind _asbp_base_chest (cast `/Game/Blueprints/Gear/Chest/BP_Base_Chest` self))
      (`/Game/Blueprints/Character/ActionCharacters/BP_Inventory.Assign Chest` _returnvalue _asbp_base_chest))
    (:`NewEnumerator2`
      (bind _asbp_base_legs (cast `/Game/Blueprints/Gear/Legs/BP_Base_Legs` self))
      (`/Game/Blueprints/Character/ActionCharacters/BP_Inventory.Assign Legs` _returnvalue _asbp_base_legs))
    (:`NewEnumerator3`
      (bind _asbp_base_weapon (cast `/Game/Blueprints/Gear/Weapon/BP_Base_Weapon` self))
      (`/Game/Blueprints/Character/ActionCharacters/BP_Inventory.Assign Weapon` _returnvalue _asbp_base_weapon)))
  (`/Game/Blueprints/Character/ActionCharacters/BP_ActionBaseCharacter.Set Stats` _linkedactioncharacter)
  (`self.K2_SetActorLocation` (0.0 0.0 -500.0))
  (bind _returnvalue_2 (`GameplayStatics.GetActorOfClass` "/Game/Blueprints/Battle/BP_BattlePhaseManager.BP_BattlePhaseManager_C"))
  (`KismetArrayLibrary.Array_RemoveItem` (`/Game/Blueprints/Battle/BP_BattlePhaseManager.Equipment To Be Destroyed` _returnvalue_2) self))

(event `self.ReceiveBeginPlay`
  (`self.Randomize Stats`)
  (`self.Set Loot Panel`)
  (`self.Set Loot Panel Vis` false))

(fn `Check Loot Panel Stats`
  (locals (CurPlayer :type "/Game/Blueprints/Character/ActionCharacters/BP_Inventory Object Reference"))
  (bind _gear_atk (`self.Gear_ATK`))
  (bind _gear_def (`self.Gear_DEF`))
  (bind _gear_spd (`self.Gear_SPD`))
  (bind (_s_gear_icon _s_gear_name _s_gear_geartype) (break `/Game/Blueprints/Gear/S_GearBase` (`self.S_Gear`)))
  (bind _gear_hp (`self.Gear_HP`))
  (bind _asbp_board_game_mode (cast `/Game/Blueprints/BP_BoardGameMode` (`GameplayStatics.GetGameMode`)))
  (bind _curplayerturn (`/Game/Blueprints/BP_BoardGameMode.CurPlayerTurn` _asbp_board_game_mode))
  (`/Engine/EditorBlueprintResources/StandardMacros.IsValid` _curplayerturn
    (:`Is Valid`
      (bind _output_get (set `local.CurPlayer` (`self.GetComponentByClass` (`/Game/Blueprints/Character/BoardCharacters/BP_BoardBaseCharacter.LinkedActionCharacter` _curplayerturn) "/Game/Blueprints/Character/ActionCharacters/BP_Inventory.BP_Inventory_C")))
      (switch `/Game/Blueprints/Gear/E_GearType` _s_gear_geartype
        (:`NewEnumerator0`
          (bind _head_slot (`/Game/Blueprints/Character/ActionCharacters/BP_Inventory.Head Slot` _output_get))
          (`self.Set Compare Text` (`/Game/Blueprints/Gear/BP_Base_Equipment.Gear_ATK` _head_slot) _gear_atk (`self.ATK Compare`))
          (`self.Set Compare Text` (`/Game/Blueprints/Gear/BP_Base_Equipment.Gear_DEF` _head_slot) _gear_def (`self.DEF Compare`))
          (`self.Set Compare Text` (`/Game/Blueprints/Gear/BP_Base_Equipment.Gear_SPD` _head_slot) _gear_spd (`self.SPD Compare`))
          (`self.Set Compare Text` (`/Game/Blueprints/Gear/BP_Base_Equipment.Gear_HP` _head_slot) _gear_hp (`self.HP Compare`)))
        (:`NewEnumerator1`
          (bind _chest_slot (`/Game/Blueprints/Character/ActionCharacters/BP_Inventory.Chest Slot` _output_get))
          (`self.Set Compare Text` (`/Game/Blueprints/Gear/BP_Base_Equipment.Gear_ATK` _chest_slot) _gear_atk (`self.ATK Compare`))
          (`self.Set Compare Text` (`/Game/Blueprints/Gear/BP_Base_Equipment.Gear_DEF` _chest_slot) _gear_def (`self.DEF Compare`))
          (`self.Set Compare Text` (`/Game/Blueprints/Gear/BP_Base_Equipment.Gear_SPD` _chest_slot) _gear_spd (`self.SPD Compare`))
          (`self.Set Compare Text` (`/Game/Blueprints/Gear/BP_Base_Equipment.Gear_HP` _chest_slot) _gear_hp (`self.HP Compare`)))
        (:`NewEnumerator2`
          (bind _leg_slot (`/Game/Blueprints/Character/ActionCharacters/BP_Inventory.Leg Slot` _output_get))
          (`self.Set Compare Text` (`/Game/Blueprints/Gear/BP_Base_Equipment.Gear_ATK` _leg_slot) _gear_atk (`self.ATK Compare`))
          (`self.Set Compare Text` (`/Game/Blueprints/Gear/BP_Base_Equipment.Gear_DEF` _leg_slot) _gear_def (`self.DEF Compare`))
          (`self.Set Compare Text` (`/Game/Blueprints/Gear/BP_Base_Equipment.Gear_SPD` _leg_slot) _gear_spd (`self.SPD Compare`))
          (`self.Set Compare Text` (`/Game/Blueprints/Gear/BP_Base_Equipment.Gear_HP` _leg_slot) _gear_hp (`self.HP Compare`)))
        (:`NewEnumerator3`
          (bind _weapon_slot (`/Game/Blueprints/Character/ActionCharacters/BP_Inventory.Weapon Slot` _output_get))
          (`self.Set Compare Text` (`/Game/Blueprints/Gear/BP_Base_Equipment.Gear_ATK` _weapon_slot) _gear_atk (`self.ATK Compare`))
          (`self.Set Compare Text` (`/Game/Blueprints/Gear/BP_Base_Equipment.Gear_DEF` _weapon_slot) _gear_def (`self.DEF Compare`))
          (`self.Set Compare Text` (`/Game/Blueprints/Gear/BP_Base_Equipment.Gear_SPD` _weapon_slot) _gear_spd (`self.SPD Compare`))
          (`self.Set Compare Text` (`/Game/Blueprints/Gear/BP_Base_Equipment.Gear_HP` _weapon_slot) _gear_hp (`self.HP Compare`))))
      (bind _asloot_panel (cast `/Game/Blueprints/Gear/LootPanel` (`WidgetComponent.GetUserWidgetObject` (`self.Widget`))))
      (set `/Game/Blueprints/Gear/LootPanel.ATK Compare` (`KismetTextLibrary.Conv_StringToText` (`self.ATK Compare`)) _asloot_panel)
      (set `/Game/Blueprints/Gear/LootPanel.DEF Compare` (`KismetTextLibrary.Conv_StringToText` (`self.DEF Compare`)) _asloot_panel)
      (set `/Game/Blueprints/Gear/LootPanel.SPD Compare` (`KismetTextLibrary.Conv_StringToText` (`self.SPD Compare`)) _asloot_panel)
      (set `/Game/Blueprints/Gear/LootPanel.HP Compare` (`KismetTextLibrary.Conv_StringToText` (`self.HP Compare`)) _asloot_panel))))

(fn `GetGearTotalAmount`
  (returns (Amount :type Integer))
  (return (+ (`self.Gear_HP`) (`self.Gear_ATK`) (`self.Gear_DEF`) (`self.Gear_SPD`))))

(fn `Randomize Stats`
  (set `self.Gear_HP` (`KismetMathLibrary.RandomIntegerInRange` (`self.Gear_HP_Range_Min`) (`self.Gear_HP_Range_Max`)))
  (set `self.Gear_ATK` (`KismetMathLibrary.RandomIntegerInRange` (`self.Gear_ATK_Range_Min`) (`self.Gear_ATK_Range_Max`)))
  (set `self.Gear_DEF` (`KismetMathLibrary.RandomIntegerInRange` (`self.Gear_DEF_Range_Min`) (`self.Gear_DEF_Range_Max`)))
  (set `self.Gear_SPD` (`KismetMathLibrary.RandomIntegerInRange` (`self.Gear_SPD_Range_Min`) (`self.Gear_SPD_Range_Max`))))

(fn `Set Compare Text`
  (params (CurLoot :type Integer) (`New Loot` :type Integer) (`CompareStat to Change` :type "String (by ref)"))
  (if (> CurLoot `New Loot`)
    (`|VariableSetRef` `CompareStat to Change` "-")
    (elif (< CurLoot `New Loot`)
      (`|VariableSetRef` `CompareStat to Change` "+")
      (else
        (`|VariableSetRef` `CompareStat to Change` "/")))))

(fn `Set Loot Panel`
  (bind (_s_gear_icon _s_gear_name) (break `/Game/Blueprints/Gear/S_GearBase` (`self.S_Gear`)))
  (bind _asloot_panel (cast `/Game/Blueprints/Gear/LootPanel` (`WidgetComponent.GetUserWidgetObject` (`self.Widget`))))
  (set `/Game/Blueprints/Gear/LootPanel.ATK Number` (`KismetTextLibrary.Conv_IntToText` (`self.Gear_ATK`)) _asloot_panel)
  (set `/Game/Blueprints/Gear/LootPanel.DEF Number` (`KismetTextLibrary.Conv_IntToText` (`self.Gear_DEF`)) _asloot_panel)
  (set `/Game/Blueprints/Gear/LootPanel.SPD Number` (`KismetTextLibrary.Conv_IntToText` (`self.Gear_SPD`)) _asloot_panel)
  (set `/Game/Blueprints/Gear/LootPanel.HP Number` (`KismetTextLibrary.Conv_IntToText` (`self.Gear_HP`)) _asloot_panel)
  (set `/Game/Blueprints/Gear/LootPanel.Loot Name` (`KismetTextLibrary.Conv_StringToText` _s_gear_name) _asloot_panel)
  (`self.Check Loot Panel Stats`))

(fn `Set Loot Panel Vis`
  (params (Vis :type Boolean))
  (`SceneComponent.SetVisibility` (`self.Widget`) Vis false))

(fn `UserConstructionScript`)