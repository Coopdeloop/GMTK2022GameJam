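; Battle manager that runs an automatic turn-based fight between two characters, placing them at set locations on BeginPlay.
; Timed phases loop: action points accrue from SPD plus a base, reaching the threshold flags an attack, then health is checked.
; Damage scales ATK against DEF, though Attack selects the attacker as its own defender and attack flags never reset.
; Deaths end the battle, destroying dead characters and calling an empty victory hook for non-challenge Player2 defeats.
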(event `EndBattle`
  (bind _player1 (`self.Player1`))
  (bind _player2 (`self.Player2`))
  (`|ExecutionSequence`
    (:`then_0`
      (if (`/Game/Blueprints/Character/ActionCharacters/BP_ActionBaseCharacter.bIsDead` _player1)
        (`self.K2_DestroyActor` _player1)))
    (:`then_1`
      (if (`/Game/Blueprints/Character/ActionCharacters/BP_ActionBaseCharacter.bIsDead` _player2)
        (`self.K2_DestroyActor` _player2)
        (if (not (`self.bIsChallenge`))
          (`self.Battle Victory`))))))

(event `self.ReceiveBeginPlay`
  (`KismetSystemLibrary.Delay` 1.0)
  (`self.BattleStart`))

(event `BattleStart`
  (`self.K2_SetActorLocationAndRotation` (`self.Player1`) (`self.Player1Location`) (struct :`Yaw` 90.0) false false)
  (`self.K2_SetActorLocationAndRotation` (`self.Player2`) (`self.Player2Location`) (struct :`Yaw` -90.0) false false)
  (`KismetSystemLibrary.Delay` 2.0)
  (`self.CalculateTurnStats`))

(event `CalculateTurnStats`
  (`KismetSystemLibrary.PrintString` "Adding Action Points")
  (`self.AddActionPoints`)
  (`self.CheckIfCanAction`)
  (`KismetSystemLibrary.Delay` 1.0)
  (`self.AttackPhase`))

(event `AttackPhase`
  (`KismetSystemLibrary.PrintString` "Attack Phase")
  (`|ExecutionSequence`
    (:`then_0`
      (if (`self.bPlayer1Attacking`)
        (`self.Attack` (`self.Player1`))
        (set `self.Player1ActionPoints` 0)))
    (:`then_1`
      (if (`self.bPlayer2Attacking`)
        (`self.Attack` (`self.Player2`))
        (set `self.Player2ActionPoints` 0)))
    (:`then_2`
      (`KismetSystemLibrary.Delay` 2.0)
      (`self.CalcHitDamagePhase`))))

(event `CalcHitDamagePhase`
  (`self.CheckHealth`))

(fn `AddActionPoints`
  (set `self.Player1ActionPoints` (+ (`/Game/Blueprints/Character/ActionCharacters/BP_ActionBaseCharacter.SPD` (`self.Player1`)) (`self.BaseActionPointsAdded`) (`self.Player1ActionPoints`)))
  (set `self.Player2ActionPoints` (+ (`/Game/Blueprints/Character/ActionCharacters/BP_ActionBaseCharacter.SPD` (`self.Player2`)) (`self.BaseActionPointsAdded`) (`self.Player1ActionPoints`))))

(fn `Attack`
  (params (AttackingPlayer :type "/Game/Blueprints/Character/ActionCharacters/BP_ActionBaseCharacter Object Reference"))
  (locals (DefendingPlayer :type "/Game/Blueprints/Character/ActionCharacters/BP_ActionBaseCharacter Object Reference") (DamageDone :type Integer))
  (bind _defendingplayer (`local.DefendingPlayer`))
  (bind _returnvalue (`KismetMathLibrary.Conv_IntToDouble` (`/Game/Blueprints/Character/ActionCharacters/BP_ActionBaseCharacter.ATK` AttackingPlayer)))
  (bind _output_get (set `local.DefendingPlayer` (select `bool` (== AttackingPlayer (`self.Player1`)) :`false` (`self.Player2`) :`true` (`self.Player1`))))
  (bind _output_get_2 (set `local.DamageDone` (`KismetMathLibrary.FCeil` (/ (* _returnvalue _returnvalue) (+ _returnvalue (`KismetMathLibrary.Conv_IntToDouble` (`/Game/Blueprints/Character/ActionCharacters/BP_ActionBaseCharacter.DEF` _output_get)))))))
  (bind _returnvalue_2 (- (`/Game/Blueprints/Character/ActionCharacters/BP_ActionBaseCharacter.HP` _defendingplayer) _output_get_2))
  (set `/Game/Blueprints/Character/ActionCharacters/BP_ActionBaseCharacter.HP` (`KismetMathLibrary.SelectInt` 0 _returnvalue_2 (< _returnvalue_2 0)) _defendingplayer))

(fn `Battle Victory`)

(fn `CheckHealth`
  (bind _bisdead (`/Game/Blueprints/Character/ActionCharacters/BP_ActionBaseCharacter.bIsDead` (`self.Player1`)))
  (bind _bisdead_2 (`/Game/Blueprints/Character/ActionCharacters/BP_ActionBaseCharacter.bIsDead` (`self.Player2`)))
  (`|ExecutionSequence`
    (:`then_0`
      (if (<= (`/Game/Blueprints/Character/ActionCharacters/BP_ActionBaseCharacter.HP` (`self.Player1`)) 0)
        (set `/Game/Blueprints/Character/ActionCharacters/BP_ActionBaseCharacter.bIsDead` true (`self.Player1`))))
    (:`then_1`
      (if (<= (`/Game/Blueprints/Character/ActionCharacters/BP_ActionBaseCharacter.HP` (`self.Player2`)) 0)
        (set `/Game/Blueprints/Character/ActionCharacters/BP_ActionBaseCharacter.bIsDead` true (`self.Player2`))))
    (:`then_2`
      (if (and _bisdead _bisdead_2)
        (`KismetSystemLibrary.PrintString` "Draw Logic")
        (`self.EndBattle` :!label _label)
        (elif _bisdead_2
          (`KismetSystemLibrary.PrintString` "Player 1 Wins")
          (goto _label)
          (elif _bisdead
            (`KismetSystemLibrary.PrintString` "Player 2 Wins")
            (goto _label)
            (else
              (`self.CalculateTurnStats`))))))))

(fn `CheckIfCanAction`
  (`|ExecutionSequence`
    (:`then_0`
      (if (>= (`self.Player1ActionPoints`) (`self.ActionRequirementAmount`))
        (set `self.bPlayer1Attacking` true)))
    (:`then_1`
      (if (>= (`self.Player2ActionPoints`) (`self.ActionRequirementAmount`))
        (set `self.bPlayer2Attacking` true)))))

(fn `PrepareToAttack`
  (params (CharacterPreparingToAttack :type "/Game/Blueprints/Character/ActionCharacters/BP_ActionBaseCharacter Object Reference"))
  (if (== CharacterPreparingToAttack (`self.Player1`))
    (set `self.bPlayer1Attacking` true)
    (else
      (set `self.bPlayer2Attacking` true))))

(fn `UserConstructionScript`)