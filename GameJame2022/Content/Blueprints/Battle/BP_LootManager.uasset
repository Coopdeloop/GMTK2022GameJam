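; BP_LootManager handles the loot step of a battle, offering a clickable Continue widget and hover panels for equipment.
; The widget starts hidden until TurnOnContinue shows it; clicking the actor hides it, then tells BP_BattlePhaseManager to continue the game and reset the battle.
; Tick traces under the cursor to show or hide the hovered BP_Base_Equipment's loot panel.
; BP_Base_Item is checked but gets no panel handling.
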(event `self.ReceiveActorOnClicked`
  (params (ButtonPressed :type "Key Structure"))
  (`self.Continue`))

(event `Continue`
  (bind _battlephasemanager (`self.BattlePhaseManager`))
  (`/Game/Blueprints/Battle/BP_BattlePhaseManager.Continue game` _battlephasemanager)
  (`SceneComponent.SetVisibility` (`self.Widget`) false false)
  (`/Game/Blueprints/Battle/BP_BattlePhaseManager.ResetBattle` _battlephasemanager))

(event `self.ReceiveBeginPlay`
  (bind _returnvalue (`GameplayStatics.GetActorOfClass` "/Game/Blueprints/Battle/BP_BattlePhaseManager.BP_BattlePhaseManager_C"))
  (set `self.BattlePhaseManager` _returnvalue)
  (`SceneComponent.SetVisibility` (`self.Widget`) false false))

(event `self.ReceiveTick`
  (params (DeltaSeconds :type "Float (single-precision)"))
  (bind _current_hover (`self.Current Hover`))
  (bind (_bblockinghit _binitialoverlap _time _distance _location _impactpoint _normal _impactnormal _physmat _hitactor) (`GameplayStatics.BreakHitResult` (`PlayerController.GetHitResultUnderCursorByChannel` (`GameplayStatics.GetPlayerController` 0) "TraceTypeQuery1" true)))
  (bind _returnvalue (`GameplayStatics.GetObjectClass` _hitactor))
  (if (`KismetMathLibrary.ClassIsChildOf` _returnvalue "/Game/Blueprints/Gear/BP_Base_Equipment.BP_Base_Equipment_C")
    (bind _output_get (set `self.Current Hover` _hitactor))
    (bind _asbp_base_equipment (cast `/Game/Blueprints/Gear/BP_Base_Equipment` _output_get))
    (`/Game/Blueprints/Gear/BP_Base_Equipment.Set Loot Panel Vis` _asbp_base_equipment true)
    (elif (not (`KismetMathLibrary.ClassIsChildOf` _returnvalue "/Game/Blueprints/Items/BP_Base_Item.BP_Base_Item_C"))
      (bind _asbp_base_equipment_2 (cast `/Game/Blueprints/Gear/BP_Base_Equipment` _current_hover)
        (:`then`
          (`/Game/Blueprints/Gear/BP_Base_Equipment.Set Loot Panel Vis` _asbp_base_equipment_2 false)
          (set `self.Current Hover` null))
        (:`CastFailed`
          (cast `/Game/Blueprints/Items/BP_Base_Item` _current_hover))))))

(fn `Turn On Continue`
  (`SceneComponent.SetVisibility` (`self.Widget`) true false))

(fn `UserConstructionScript`)